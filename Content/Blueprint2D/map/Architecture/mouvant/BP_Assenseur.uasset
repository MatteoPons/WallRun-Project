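; Moving elevator actor for the 2D map's architecture, which animates itself as soon as play begins.
; BeginPlay calls Bouger, which plays the Mouvement timeline and uses its float as a lerp alpha.
; A FlipFlop on the timeline update alternates on successive updates between scaling from Origine to Fin and moving from OrigineDéplacement to FinDéplacement, without sweep.
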(event `self.ReceiveBeginPlay`
  (`self.bouger`))

(event `bouger`
  (bind (_direction _float) (`Timeline|Mouvement`)
    (:`Update`
      (`/Engine/EditorBlueprintResources/StandardMacros.FlipFlop`
        (:`A`
          (`self.SetActorScale3D` (`KismetMathLibrary.VLerp` (`self.Origine`) (`self.Fin`) _float)))
        (:`B`
          (`self.K2_SetActorLocation` (`KismetMathLibrary.VLerp` (`self.OrigineDéplacement`) (`self.FinDéplacement`) _float)))))))

(fn `UserConstructionScript`)