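; BP_MurAPiquesMouvant is a moving spiked wall hazard that kills the player on contact.
; On BeginPlay, Bouger plays the Mouvement timeline, which lerps the actor's location from Origine to Fin without sweep.
; When a BP_Personnage begins overlapping the Box, it sets EnVie to false and calls Mort on that character.
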(event `self.ReceiveBeginPlay`
  (`self.bouger`))

(event `bouger`
  (bind (_direction _float) (`Timeline|Mouvement`)
    (:`Update`
      (`self.K2_SetActorLocation` (`KismetMathLibrary.VLerp` (`self.Origine`) (`self.Fin`) _float)))))

(event `self.Box.OnComponentBeginOverlap`
  (params (OverlappedComponent :type "PrimitiveComponent Object Reference") (OtherActor :type "Actor Object Reference") (OtherComp :type "PrimitiveComponent Object Reference") (OtherBodyIndex :type Integer) (bFromSweep :type Boolean) (SweepResult :type "HitResult Structure (by ref)"))
  (bind _asbp_personnage (cast `/Game/Blueprint2D/Personnage/BP_Personnage` OtherActor))
  (set `/Game/Blueprint2D/Personnage/BP_Personnage.En vie` false _asbp_personnage)
  (`/Game/Blueprint2D/Personnage/BP_Personnage.Mort` _asbp_personnage))

(fn `UserConstructionScript`)